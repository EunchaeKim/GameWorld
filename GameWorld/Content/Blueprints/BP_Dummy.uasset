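; BP_Dummy is a damageable target character with a health bar and a stealth back-assassination prompt.
; Both widgets face the camera on Tick, and the prompt appears when a crouched player enters AssasinationRadius.
; Damage plays a random hit montage and sound, launches the dummy along player forward, and updates health through BPCNPCStats.
; StealthBackAssasin plays the victim animation and returns alignment location and rotation, while Ragdoll enables delayed mesh physics.
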(event OnComponentBeginOverlap(AssasinationRadius)
  (params (OverlappedComponent :type Primitive%20Component%20Object%20Reference) (OtherActor :type Actor%20Object%20Reference) (OtherComp :type Primitive%20Component%20Object%20Reference) (OtherBodyIndex :type Integer) (bFromSweep :type Boolean) (SweepResult :type Hit%20Result%20Structure%20%28by%20ref%29))
  (bind _asbp_third_person_character_main (Utilities|Casting|CastToBP_ThirdPersonCharacter_Main OtherActor))
  (if (Variables|/Script/Engine.Character|GetbIsCrouched _asbp_third_person_character_main)
    (Rendering|SetVisibility (Variables|Default|GetAssasinate%20Widget) true false)))

(event OnComponentEndOverlap(AssasinationRadius)
  (params (OverlappedComponent :type Primitive%20Component%20Object%20Reference) (OtherActor :type Actor%20Object%20Reference) (OtherComp :type Primitive%20Component%20Object%20Reference) (OtherBodyIndex :type Integer))
  (Utilities|Casting|CastToBP_ThirdPersonCharacter_Main OtherActor)
  (Rendering|SetVisibility (Variables|Default|GetAssasinate%20Widget) false false))

(event Custom|Ragdoll
  (Utilities|FlowControl|Delay 2.5)
  (Physics|SetSimulatePhysics (Variables|Character|GetMesh) true))

(event EventBeginPlay
  (bind _bpc_npcstats (Variables|Default|GetBPC_NPCStats))
  (bind _aswb_dummy_health (Utilities|Casting|CastToWB_DummyHealth (UserInterface|GetUserWidgetObject (Variables|Default|GetHealth%20Bar%20Widget))))
  (bind _output_get (Variables|Default|SetDummyHealth%20Widget _aswb_dummy_health))
  (Default|SetHealthUIPercentandText _output_get (Default|GetCurrentHealth _bpc_npcstats) (Default|GetCurrentMaxHealth _bpc_npcstats)))

(event EventTick
  (params (DeltaSeconds :type Float%20%28single-precision%29))
  (Transformation|SetWorldRotation (Variables|Default|GetAssasinate%20Widget) (Math|Rotator|FindLookatRotation (Transformation|GetWorldLocation (Variables|Default|GetAssasinate%20Widget)) (Transformation|GetWorldLocation (Variables|/Script/Engine.PlayerCameraManager|GetTransformComponent (Game|GetPlayerCameraManager 0)))) false false))

(event Game|Damage|EventAnyDamage
  (params (Damage :type Float%20%28single-precision%29) (DamageType :type Damage%20Type%20Object%20Reference) (InstigatedBy :type Controller%20Object%20Reference) (DamageCauser :type Actor%20Object%20Reference))
  (Animation|PlayAnimMontage (Utilities|Array|Get(acopy) (Variables|Default|GetHit%20Aims) (Math|Random|RandomIntegerinRange 0 (- (Utilities|Array|Length (Variables|Default|GetHit%20Aims)) 1))) 1.0 "None")
  (bind _asbp_third_person_character_main (Utilities|Casting|CastToBP_ThirdPersonCharacter_Main (Game|GetPlayerCharacter 0)))
  (Character|LaunchCharacter (* (Math|Vector|GetForwardVector (Transformation|GetActorRotation _asbp_third_person_character_main)) 7e+02) false false)
  (Audio|PlaySoundatLocation "/Game/Audio/Grunts-Hits/Death1.Death1" (Transformation|GetActorLocation) "0, 0, 0" 1.0 (Math|Random|RandomFloatinRange -1.5 1.3) 0.0 "/Game/Audio/SA_Character.SA_Character" 0 0 0)
  (bind _current_health (Default|DecreaseHealth (Variables|Default|GetBPC_NPCStats) Damage))
  (Default|SetHealthUIPercentandText (Variables|Default|GetDummyHealth%20Widget) _current_health (Variables|/Game/Blueprints/BPC_NPCStats.BPC_NPCStats_C|GetMax%20Health (Variables|Default|GetBPC_NPCStats))))

(fn ConstructionScript)

(fn StealthBackAssasin
  (Components|Animation|PlayAnimation (Variables|Character|GetMesh) "/Game/Characters/GameCharacter/Animations/Assasination/Paired_Knife_Stealth_KidneyAndNeck_Vic1.Paired_Knife_Stealth_KidneyAndNeck_Vic1" false)
  (Rendering|SetVisibility (Variables|Default|GetAssasinate%20Widget) false false)
  (return (Transformation|GetWorldLocation (Variables|Default|GetAssasin%20REF)) (Transformation|GetActorRotation)))