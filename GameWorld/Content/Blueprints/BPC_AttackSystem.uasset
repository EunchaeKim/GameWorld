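; Attack component for BP_ThirdPersonCharacter_Main that runs a four-step melee combo of sword and kick montages from IA_Attack input.
; Presses during an attack are buffered in SaveAttack, and SwordAttackCombo either plays the next step by AttackIndex or resets the combo.
; Separate start/stop events control a looping timer that sphere-traces between the sword's two points with debug drawing; hit results are unused.
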(event Custom|SwordAttack
  ;[0.05098 0.05098 0.05098] Combo System
  ;;[0.05098 0.05098 0.05098] Sword Attack
  (if (Variables|Default|GetIs%20Attacking?)
    (Variables|Default|SetSave%20Attack? true)
    (else
      (Variables|Default|SetIs%20Attacking? true)
      (switch int (Variables|Default|GetAttack%20Index)
        (:0
          (CallFunction|Attack1))
        (:1
          (CallFunction|Attack2))
        (:2
          (CallFunction|Attack3))
        (:3
          (CallFunction|Attack4))))))

(event Custom|Sword%20Attack%20Combo
  ;[0.05098 0.05098 0.05098] Combo System
  ;;[0.05098 0.05098 0.05098] Combo Continue
  (if (Variables|Default|GetSave%20Attack?)
    (Variables|Default|SetSave%20Attack? false)
    (switch int (Variables|Default|GetAttack%20Index)
      (:0
        (CallFunction|Attack1))
      (:1
        (CallFunction|Attack2))
      (:2
        (CallFunction|Attack3))
      (:3
        (CallFunction|Attack4)))
    (else
      (CallFunction|StopCombo))))

(event Custom|Stop%20Combo
  ;[0.05098 0.05098 0.05098] Combo System
  ;;[0.05098 0.05098 0.05098] Stop Combo / Attack
  (Variables|Default|SetIs%20Attacking? false)
  (Variables|Default|SetAttack%20Index 0))

(event Custom|Attack%204
  ;[0.05098 0.05098 0.05098] Combo System
  ;;[0.05098 0.05098 0.05098] Attack 4
  (Utilities|FlowControl|DoOnce false :!label _label
    (:Completed
      (Utilities|FlowControl|Delay 0.1)
      (Animation|Montage|PlayMontage (Variables|Default|GetCharacter%20Mesh) "/Game/Characters/GameCharacter/Animations/SwordAttacks/Attack3_Montage.Attack3_Montage"
        (:then
          (Variables|Default|SetAttack%20Index 4)
          (goto _label Reset))))))

(event Custom|Attack1
  ;[0.05098 0.05098 0.05098] Combo System
  ;;[0.05098 0.05098 0.05098] Attack 1
  (Utilities|FlowControl|DoOnce false :!label _label
    (:Completed
      (Utilities|FlowControl|Delay 0.1)
      (Animation|Montage|PlayMontage (Variables|Default|GetCharacter%20Mesh) "/Game/Characters/GameCharacter/Animations/SwordAttacks/Attack1_Montage.Attack1_Montage"
        (:then
          (Variables|Default|SetAttack%20Index 1)
          (goto _label Reset))))))

(event Custom|Start%20Sword%20Trace
  (bind _returnvalue (Utilities|Time|SetTimerbyEvent (delegate Custom|Sword%20Trace%20Loop) 0.001 true))
  (Variables|Default|SetSwordTraceLoop _returnvalue))

(event Custom|Attack2
  ;[0.05098 0.05098 0.05098] Combo System
  ;;[0.05098 0.05098 0.05098] Attack 2
  (Utilities|FlowControl|DoOnce false :!label _label
    (:Completed
      (Utilities|FlowControl|Delay 0.1)
      (Animation|Montage|PlayMontage (Variables|Default|GetCharacter%20Mesh) "/Game/Characters/GameCharacter/Animations/SwordAttacks/Attack2_Montage.Attack2_Montage"
        (:then
          (Variables|Default|SetAttack%20Index 2)
          (goto _label Reset))))))

(event Custom|Sword%20Trace%20Loop
  (Collision|SphereTraceByChannel (Transformation|GetWorldLocation (Variables|/Game/ThirdPerson/Blueprints/BP_ThirdPersonCharacter_Main.BP_ThirdPersonCharacter_Main_C|GetSword%20Top%20Point (Variables|Default|GetCharacter%20BP))) (Transformation|GetWorldLocation (Variables|/Game/ThirdPerson/Blueprints/BP_ThirdPersonCharacter_Main.BP_ThirdPersonCharacter_Main_C|GetSword%20Bottom%20Point (Variables|Default|GetCharacter%20BP))) 12.0 "TraceTypeQuery1" false 0 "ForDuration" true "(R=1.000000,G=0.000000,B=0.000000,A=1.000000)" "(R=0.000000,G=1.000000,B=0.000000,A=1.000000)" 0.2))

(event Custom|Attack3
  ;[0.05098 0.05098 0.05098] Combo System
  ;;[0.05098 0.05098 0.05098] Attack 3
  (Utilities|FlowControl|DoOnce false :!label _label
    (:Completed
      (Utilities|FlowControl|Delay 0.1)
      (Animation|Montage|PlayMontage (Variables|Default|GetCharacter%20Mesh) "/Game/Characters/GameCharacter/Animations/SwordAttacks/Kick_Montage.Kick_Montage"
        (:then
          (Variables|Default|SetAttack%20Index 3)
          (goto _label Reset))))))

(event Custom|Stop%20Sword%20Trace
  (Utilities|Time|ClearandInvalidateTimerbyHandle (Variables|Default|GetSwordTraceLoop)))

(event Input|EnhancedActionEvents|EnhancedInputActionIA_Attack
  (params (ActionValue :type Boolean) (ElapsedSeconds :type Float%20%28double-precision%29) (TriggeredSeconds :type Float%20%28double-precision%29) (InputAction :type Input%20Action%20Object%20Reference :default "/Game/ThirdPerson/Input/Actions/IA_Attack.IA_Attack"))
  ;[0.05098 0.05098 0.05098] Combo System
  ;;[0.05098 0.05098 0.05098] Attack Input
  (:Started
    (if (Variables|Default|GetCan%20Attack?)
      (CallFunction|SwordAttack))))

(event EventBeginPlay
  (bind _asbp_third_person_character_main (Utilities|Casting|CastToBP_ThirdPersonCharacter_Main (Components|GetOwner)))
  (Variables|Default|SetCharacter%20BP _asbp_third_person_character_main)
  (Variables|Default|SetCharacter%20Mesh (Variables|/Script/Engine.Character|GetMesh _asbp_third_person_character_main)))