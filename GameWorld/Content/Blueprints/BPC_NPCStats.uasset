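; BPC_NPCStats is a component that holds an NPC's health and stamina.
; Functions lower current values with a floor at zero, raise them capped at their maximums, and increase the maximums.
; DecreaseHealth returns a death flag and the remaining health, and getters expose current and maximum health.
; The component updates no UI, as its BeginPlay is empty and the BP_Dummy health bar nodes are disconnected.
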(event EventBeginPlay)

(fn DecreaseHealth
  (params (Damage :type Float%20%28double-precision%29))
  (if (<= (- (Variables|Health|GetCurrent%20Health) Damage) 0.0)
    (Variables|Health|SetCurrent%20Health 0.0)
    (else
      (Variables|Health|SetCurrent%20Health (- (Variables|Health|GetCurrent%20Health) Damage))))
  (if (<= (Variables|Health|GetCurrent%20Health) 0.0)
    (return true (Variables|Health|GetCurrent%20Health))
    (else
      (return false (Variables|Health|GetCurrent%20Health)))))

(fn IncreaseMaxHealth
  (params (Health%20Incremention :type Float%20%28double-precision%29))
  (bind _output_get (Variables|Health|SetMax%20Health (+ (Variables|Health|GetMax%20Health) Health%20Incremention))))

(fn DecreaseStamina
  (params (Stamina%20Depleted :type Float%20%28double-precision%29))
  (if (<= (- (Variables|Stamina|GetCurrent%20Stamina) Stamina%20Depleted) 0.0)
    (Variables|Stamina|SetCurrent%20Stamina 0.0)
    (else
      (bind _output_get (Variables|Stamina|SetCurrent%20Stamina (- (Variables|Stamina|GetCurrent%20Stamina) Stamina%20Depleted))))))

(fn IncreaseMaxStamina
  (params (Added%20Stamina :type Float%20%28double-precision%29))
  (Variables|Stamina|SetMax%20Stamina (+ Added%20Stamina (Variables|Stamina|GetMax%20Stamina))))

(fn IncreaseHealth
  (params (Added%20Health :type Float%20%28double-precision%29))
  (bind _output_get (Variables|Health|SetCurrent%20Health (+ (Variables|Health|GetCurrent%20Health) Added%20Health)))
  (if (> _output_get (Variables|Health|GetMax%20Health))
    (Variables|Health|SetCurrent%20Health (Variables|Health|GetMax%20Health))))

(fn IncreaseStamina
  (params (Added%20Stamina :type Float%20%28double-precision%29))
  (Variables|Stamina|SetCurrent%20Stamina (+ Added%20Stamina (Variables|Stamina|GetCurrent%20Stamina)))
  (if (> (Variables|Stamina|GetCurrent%20Stamina) (Variables|Stamina|GetMax%20Stamina))
    (Variables|Stamina|SetCurrent%20Stamina (Variables|Stamina|GetMax%20Stamina))))

(fn GetCurrentMaxHealth
  (return (Variables|Health|GetMax%20Health)))

(fn GetCurrentHealth
  (return (Variables|Health|GetCurrent%20Health)))