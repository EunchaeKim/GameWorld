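; BP_Waypoint is a map waypoint that the player discovers by entering its range.
; The construction script sizes the DiscoverRange sphere from DiscoverRadius.
; On overlap by BP_ThirdPersonCharacter_Main, it casts the character's first child actor to BP_WorldMap and passes itself to DiscoverWaypoint.
; Its OnDiscovered event destroys the sphere component, ending further overlap detection.
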(event OnComponentBeginOverlap(DiscoverRange)
  (params (OverlappedComponent :type Primitive%20Component%20Object%20Reference) (OtherActor :type Actor%20Object%20Reference) (OtherComp :type Primitive%20Component%20Object%20Reference) (OtherBodyIndex :type Integer) (bFromSweep :type Boolean) (SweepResult :type Hit%20Result%20Structure%20%28by%20ref%29))
  (bind _asbp_third_person_character_main (Utilities|Casting|CastToBP_ThirdPersonCharacter_Main OtherActor))
  (bind _asbp_world_map (Utilities|Casting|CastToBP_WorldMap (Utilities|Array|Get(acopy) (Actor|GetAllChildActors _asbp_third_person_character_main true))))
  (Utilities|IsValid _asbp_world_map
    (:Is%20Valid
      (Default|DiscoverWaypoint _asbp_world_map self))))

(event Custom|OnDiscovered
  (Components|DestroyComponent (Variables|Default|GetDiscoverRange)))

(event EventBeginPlay)

(event Collision|EventActorBeginOverlap
  (params (OtherActor :type Actor%20Object%20Reference)))

(event EventTick
  (params (DeltaSeconds :type Float%20%28single-precision%29)))

(fn ConstructionScript
  (Components|Sphere|SetSphereRadius (Variables|Default|GetDiscoverRange) (Variables|Settings|GetDiscoverRadius) false))